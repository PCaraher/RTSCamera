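; BP_Commander is a player-controlled camera pawn with an input-driven zoom.
; BeginPlay adds the IMC_FreeMove Enhanced Input mapping context to its player controller.
; IA_CameraZoom plays or reverses the Zoom timeline by input sign and stops it on completion, allowing partial zoom.
; Timeline curves drive spring arm length and socket height, scaled by Multi, plus camera pitch, so distance, height and angle change together.
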(event `EnhancedInput|/Game/FrameWorks/Inputs/IA_CameraZoom`
  (params (ActionValue :type "Float (double-precision)") (ElapsedSeconds :type "Float (double-precision)") (TriggeredSeconds :type "Float (double-precision)") (InputAction :type "InputAction Object Reference" :default "/Game/FrameWorks/Inputs/IA_CameraZoom.IA_CameraZoom"))
  (bind _springarm (`self.SpringArm`))
  (bind _multi (`self.Multi`))
  (:`Triggered`
    (if (> ActionValue 0.0)
      (bind (_direction _cameraposition _camerarotation) (`Timeline|Zoom` :!via `Reverse` :!label _label)
        (:`Update`
          (set `SpringArmComponent.TargetArmLength` (+ 900.0 (* (.x _cameraposition) _multi)) _springarm)
          (set `SpringArmComponent.SocketOffset` (`KismetMathLibrary.MakeVector` 0.0 0.0 (* (* (.z _cameraposition) _multi) 0.5)) _springarm)
          (`SceneComponent.K2_SetRelativeRotation` (`self.Camera`) (`KismetMathLibrary.MakeRotator` 0.0 (* (.y _camerarotation) -15.0)) false false)))
      (else
        (goto _label))))
  (:`Completed`
    (goto _label :!via `Stop`)))

(event `self.ReceiveBeginPlay`
  (bind _asplayer_controller (cast `PlayerController` (`self.GetController`)))
  (message `EnhancedInputSubsystemInterface.AddMappingContext` (pcsubsystem `EnhancedInputLocalPlayerSubsystem` _asplayer_controller) "/Game/FrameWorks/Inputs/IMC_FreeMove.IMC_FreeMove" 0 (struct)))

(fn `UserConstructionScript`)