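; Player controller that drives the camera by moving and turning its possessed Commander pawn, cached on BeginPlay.
; Enhanced Input translate actions feed movement input along the pawn's forward and right vectors.
; Rotate input spins the pawn's facing vector around world Z, scaled by a rotation multiplier.
; Boost start and completion share one path that switches move speed, passed as the input scale, between default and multiplied values.
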(event `EnhancedInput|/Game/FrameWorks/Inputs/IA_CameraRotate`
  (params (ActionValue :type "Float (double-precision)") (ElapsedSeconds :type "Float (double-precision)") (TriggeredSeconds :type "Float (double-precision)") (InputAction :type "InputAction Object Reference" :default "/Game/FrameWorks/Inputs/IA_CameraRotate.IA_CameraRotate"))
  (bind _commander (`self.Commander`))
  (:`Triggered`
    (`self.K2_SetActorRotation` _commander (`KismetMathLibrary.Conv_VectorToRotator` (`KismetMathLibrary.RotateAngleAxis` (`KismetMathLibrary.Conv_RotatorToVector` (`self.K2_GetActorRotation` _commander)) (* (`self.CameraRotationMulti`) ActionValue) (0.0 0.0 1.0))) false)))

(event `EnhancedInput|/Game/FrameWorks/Inputs/IA_CameraTranslate`
  (params (ActionValue :type "Vector2D Structure") (ElapsedSeconds :type "Float (double-precision)") (TriggeredSeconds :type "Float (double-precision)") (InputAction :type "InputAction Object Reference" :default "/Game/FrameWorks/Inputs/IA_CameraTranslate.IA_CameraTranslate"))
  (bind _commander (`self.Commander`))
  (:`Triggered`
    (`Pawn.AddMovementInput` _commander (+ (* (`self.GetActorForwardVector` _commander) ActionValue_Y) (* (`self.GetActorRightVector` _commander) ActionValue_X)) (`self.CameraMoveSpeed`) false)))

(event `EnhancedInput|/Game/FrameWorks/Inputs/IA_CameraBoost`
  (params (ActionValue :type Boolean) (ElapsedSeconds :type "Float (double-precision)") (TriggeredSeconds :type "Float (double-precision)") (InputAction :type "InputAction Object Reference" :default "/Game/FrameWorks/Inputs/IA_CameraBoost.IA_CameraBoost"))
  (:`Started`
    (bind _output_get (set `self.CameraBoostToggle` ActionValue :!label _label))
    (if _output_get
      (set `self.CameraMoveSpeed` (* (`self.CameraMoveSpeedDefault`) (`self.CameraBoostMulti`)))
      (else
        (set `self.CameraMoveSpeed` (`self.CameraMoveSpeedDefault`)))))
  (:`Completed`
    (goto _label)))

(event `self.ReceiveBeginPlay`
  (set `self.Commander` (`self.K2_GetPawn`))
  (set `self.CameraMoveSpeed` (`self.CameraMoveSpeedDefault`)))

(event `self.ReceiveTick`
  (params (DeltaSeconds :type "Float (single-precision)")))

(fn `UserConstructionScript`)